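; BP_QuantumForceField is a triggerable force field that shows or hides a plane and blocks or ignores physics bodies.
; StartInactive sets the initial look and collision, and inverts how TriggereableState maps to them.
; Both open and close events share one update path for plane visibility and box collision.
; On box overlap, it releases the overlapping actor's QF_GrabComponent, but only when that mapping yields the hidden, non-blocking state.
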(event `self.ReceiveBeginPlay`
  (bind _bstartinactive (`self.bStartInactive`))
  (`SceneComponent.SetHiddenInGame` (`self.Plane`) _bstartinactive false)
  (`PrimitiveComponent.SetCollisionResponseToChannel` (`self.Box`) "ECC_PhysicsBody" (select `bool` _bstartinactive :`false` "ECR_Block" :`true` "ECR_Ignore" :!type "ECollisionResponse Enum")))

(event `self.OnTriggereableClossed`
  (bind _btriggereablestate (`self.bTriggereableState`))
  (bind _returnvalue (not (select `bool` (`self.bStartInactive`) :`false` _btriggereablestate :`true` (not _btriggereablestate))))
  (`SceneComponent.SetHiddenInGame` (`self.Plane`) _returnvalue false :!label _label)
  (`PrimitiveComponent.SetCollisionResponseToChannel` (`self.Box`) "ECC_PhysicsBody" (select `bool` _returnvalue :`false` "ECR_Block" :`true` "ECR_Ignore" :!type "ECollisionResponse Enum")))

(event `self.OnTriggereableOpened`
  (goto _label))

(event `self.Box.OnComponentBeginOverlap`
  (params (OverlappedComponent :type "PrimitiveComponent Object Reference") (OtherActor :type "Actor Object Reference") (OtherComp :type "PrimitiveComponent Object Reference") (OtherBodyIndex :type Integer) (bFromSweep :type Boolean) (SweepResult :type "HitResult Structure (by ref)"))
  (bind _returnvalue (`self.GetComponentByClass` OtherActor "/Script/QuantumField.QF_GrabComponent"))
  (bind _btriggereablestate (`self.bTriggereableState`))
  (if (not (select `bool` (`self.bStartInactive`) :`false` _btriggereablestate :`true` (not _btriggereablestate)))
    (`/Engine/EditorBlueprintResources/StandardMacros.IsValid` _returnvalue
      (:`Is Valid`
        (`QF_GrabComponent.Release` _returnvalue)))))

(fn `UserConstructionScript`)