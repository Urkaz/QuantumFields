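; A triggerable door that moves its quantum mesh between closed and open poses when it receives open and close events.
; On BeginPlay it caches the mesh's relative transform as the closed pose, while the DoorTarget component's relative transform defines the open pose.
; The DoorMovement timeline plays on open and reverses on close, with its DoorAlpha track driving a transform lerp between the two poses.
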(event `self.ReceiveBeginPlay`
  (set `self.InitialTransform` (`SceneComponent.GetRelativeTransform` (`self.QF_QuantumMesh`))))

(event `self.OnTriggereableOpened`
  (bind (_direction _dooralpha) (`Timeline|DoorMovement` :!label _label)
    (:`Update`
      (`SceneComponent.K2_SetRelativeTransform` (`self.QF_QuantumMesh`) (`KismetMathLibrary.TLerp` (`self.InitialTransform`) (`SceneComponent.GetRelativeTransform` (`self.DoorTarget`)) _dooralpha) false false))))

(event `self.OnTriggereableClossed`
  (goto _label :!via `Reverse`))

(fn `UserConstructionScript`)