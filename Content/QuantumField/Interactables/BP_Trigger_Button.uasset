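; Trigger button in QuantumField that toggles its trigger state when a valid actor begins or ends overlapping its capsule.
; CheckValidActorsForTrigger always accepts the quantum pick, and the first-person character only when ActivateOnlyOnce is off.
; The construction script creates a dynamic material on the cylinder, recolored on BeginPlay and after each toggle according to TriggerState and ActivateOnlyOnce.
; ToggleTriggerState is called but not defined here.
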(event `self.Capsule.OnComponentBeginOverlap`
  (params (OverlappedComponent :type "PrimitiveComponent Object Reference") (OtherActor :type "Actor Object Reference") (OtherComp :type "PrimitiveComponent Object Reference") (OtherBodyIndex :type Integer) (bFromSweep :type Boolean) (SweepResult :type "HitResult Structure (by ref)"))
  (bind _bactivateonlyonce (`self.bActivateOnlyOnce`))
  (if (`self.CheckValidActorsForTrigger` OtherActor)
    (`self.ToggleTriggerState` :!label _label)
    (`MaterialInstanceDynamic.SetVectorParameterValue` (`self.DynamicMaterialTest`) "Color" (`KismetMathLibrary.SelectColor` (`KismetMathLibrary.SelectColor` (struct :`R` 1.0 :`G` 0.966577 :`A` 1.0) (struct :`R` 0.003922 :`G` 1.0 :`B` 0.109804 :`A` 1.0) _bactivateonlyonce) (`KismetMathLibrary.SelectColor` (struct :`G` 0.041792 :`B` 1.0 :`A` 1.0) (struct :`R` 1.0 :`G` 0.090196 :`A` 1.0) _bactivateonlyonce) (`self.bTriggerState`)) :!label _label_2)))

(event `self.ReceiveBeginPlay`
  (goto _label_2))

(event `self.Capsule.OnComponentEndOverlap`
  (params (OverlappedComponent :type "PrimitiveComponent Object Reference") (OtherActor :type "Actor Object Reference") (OtherComp :type "PrimitiveComponent Object Reference") (OtherBodyIndex :type Integer))
  (if (`self.CheckValidActorsForTrigger` OtherActor)
    (goto _label)))

(fn `CheckValidActorsForTrigger`
  (params (Object :type "Object Object Reference"))
  (returns (ReturnValue :type Boolean))
  (bind _returnvalue (`GameplayStatics.GetObjectClass` Object))
  (if (== _returnvalue "/Game/Developers/Juanjo/BP_QF_QuantumPick.BP_QF_QuantumPick_C")
    _
    (elif (and (== _returnvalue "/Game/FirstPerson/Blueprints/BP_FirstPersonCharacter.BP_FirstPersonCharacter_C") (not (`self.bActivateOnlyOnce`)))
      _
      (else
        (return false))))
  (return true))

(fn `UserConstructionScript`
  (bind _returnvalue (`PrimitiveComponent.CreateDynamicMaterialInstance` (`self.Cylinder`) 0 "/Engine/BasicShapes/BasicShapeMaterial.BasicShapeMaterial" "None"))
  (set `self.DynamicMaterialTest` _returnvalue))