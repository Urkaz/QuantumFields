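; Quantum field sphere that animates its growth and collapse, with create and cancel sounds.
; Separate timelines for activate, finish, interrupt and both deactivation stages drive scale updates and the material's opacity, refraction and noise, with collapse timelines played in reverse.
; Only the initial activation checks overlaps; timeline completion sends end-activate, end-deactivate or destroy notifications.
; Interrupting stops activation and blocks its end notification; an older combined timeline remains unconnected.
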(event `self.BP_SphereActivate`
  ;[1 0.9489 0] Activate
  (`self.PlaySphereSound` false)
  (bind (_direction _scalemultiplier _opacityfalloff _refractionindex) (`Timeline|ActivateTimeline` :!via `PlayFromStart` :!label _label)
    (:`Update`
      (`self.Update_Activating` _scalemultiplier true)
      (`self.Update Material Parameters` _opacityfalloff _refractionindex))
    (:`Finished`
      (if (not (`self.BlockEndNotifications`))
        (`self.TryNotifyEndActivate`)))))

(event `StopActivateTimelines`
  (`|ExecutionSequence`
    (:`then_0`
      (goto _label :!via `Stop`))
    (:`then_1`
      ;[0.1065 1 0] Finished Activating
      (bind (_direction _scalemultiplier _opacityfalloff _refractionindex) (`Timeline|FinishActivateTimeline` :!via `Stop` :!label _label_2)
        (:`Update`
          (`self.Update_Activating` _scalemultiplier)
          (`self.Update Material Parameters` _opacityfalloff _refractionindex))
        (:`Finished`
          (`MaterialInstanceDynamic.SetScalarParameterValue` (`self.SphereMaterialInstance`) "MinOpacity" 0.0))))))

(event `self.BP_SphereFinishedActivating`
  ;[0.1065 1 0] Finished Activating
  (goto _label_2 :!via `PlayFromStart`))

(event `self.BP_SphereInterruptActivate`
  ;[1 0.3062 0] Interrupt
  (set `self.BlockEndNotifications` true)
  (`self.StopActivateTimelines`)
  (`self.PlaySphereSound` true)
  (bind (_direction _scalemultiplier _opacityfalloff _refractionindex) (`Timeline|InterruptTimeline` :!via `ReverseFromEnd`)
    (:`Update`
      (`self.Update_Deactivating` _scalemultiplier)
      (`self.Update Material Parameters` _opacityfalloff _refractionindex))
    (:`Finished`
      (`self.TryNotifyEndDeactivate`))))

(event `PlaySphereSound`
  (params (bDelete :type Boolean))
  ;[0 0.3203 1] Audio
  (`GameplayStatics.PlaySoundAtLocation` (select `bool` bDelete :`false` "/Game/QuantumField/Sound/MetaSounds/sound/CreateSphere/CreateSphere_CUE.CreateSphere_CUE" :`true` "/Game/QuantumField/Sound/MetaSounds/sound/CancelSphere/CancelSphere_CUE.CancelSphere_CUE" :!type "SoundBase Object Reference") (`self.K2_GetActorLocation`) (struct) 1.0 1.0 0.0 null null null null))

(event `self.BP_SphereDeactivate`
  ;[1 0 0] Deactivate
  (`self.PlaySphereSound` true)
  (bind (_direction _scalemultiplier _opacityfalloff _refractionindex) (`Timeline|DeactivateTimeline` :!via `ReverseFromEnd`)
    (:`Update`
      (`self.Update_Deactivating` _scalemultiplier)
      (`self.Update Material Parameters` _opacityfalloff _refractionindex))
    (:`Finished`
      (`self.TryNotifyEndDeactivate`))))

(event `self.BP_SphereFinishedDeactivating`
  ;[0.1469 0.1469 0.1469] Finished Deactivating
  (bind (_direction _scalemultiplier _opacityfalloff _refractionindex) (`Timeline|FinishedDeactivatingTimeline` :!via `ReverseFromEnd`)
    (:`Update`
      (`self.Update_Deactivating` _scalemultiplier)
      (`self.Update Material Parameters` _opacityfalloff _refractionindex))
    (:`Finished`
      (`self.NotifyDestroy`))))

(fn `Update Material Parameters`
  (params (Opacity :type "Float (single-precision)") (refraction :type "Float (single-precision)"))
  (bind _spherematerialinstance (`self.SphereMaterialInstance`))
  (`MaterialInstanceDynamic.SetScalarParameterValue` _spherematerialinstance "MinOpacity" (* Opacity 100.0))
  (`MaterialInstanceDynamic.SetScalarParameterValue` _spherematerialinstance "RefractionIndex" refraction)
  (`MaterialInstanceDynamic.SetScalarParameterValue` _spherematerialinstance "DisableNoise" Opacity))

(fn `UserConstructionScript`)